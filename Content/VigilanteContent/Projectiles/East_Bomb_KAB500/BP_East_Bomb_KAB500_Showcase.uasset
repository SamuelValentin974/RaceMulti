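; Showcase Blueprint for the East KAB-500 bomb that exposes its fins for interactive posing.
; Four slider events each pass their value to the matching fin angle setter, so each of the four fins is adjusted independently.
; The construction script only calls its parent, and the default BeginPlay, overlap and Tick events are disabled.
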(event EventBeginPlay
  (|CallParentFunction) ; This node is disabled and will not be called.\nDrag off pins to build functionality.
)

(event Collision|EventActorBeginOverlap
  (params (OtherActor :type Actor%20Object%20Reference))
  (|CallParentFunction OtherActor) ; This node is disabled and will not be called.\nDrag off pins to build functionality.
)

(event EventTick
  (params (DeltaSeconds :type Float%20%28single-precision%29))
  (|CallParentFunction DeltaSeconds) ; This node is disabled and will not be called.\nDrag off pins to build functionality.
)

(event EventSetSliderVariable0
  (params (NewValue :type Float%20%28single-precision%29))
  (CallFunction|SetFin1Angle NewValue))

(event EventSetSliderVariable1
  (params (NewValue :type Float%20%28single-precision%29))
  (CallFunction|SetFin2Angle NewValue))

(event EventSetSliderVariable2
  (params (NewValue :type Float%20%28single-precision%29))
  (CallFunction|SetFin3Angle NewValue))

(event EventSetSliderVariable3
  (params (NewValue :type Float%20%28single-precision%29))
  (CallFunction|SetFin4Angle NewValue))

(fn ConstructionScript
  (|CallParentFunction))