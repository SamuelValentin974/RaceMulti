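; Blueprint for the East KAB-500 bomb, exposing animated control of its four fins.
; On BeginPlay it casts and caches the skeletal mesh's BPA_East_Bomb_KAB500 anim instance.
; One event per fin takes a normalized -1 to 1 input, remaps it with clamping to a ±45 range, and writes it to that anim instance's matching fin angle variable.
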(event Custom|SetFin1Angle
  (params (Fin1Angle :type Float%20%28single-precision%29))
  (Variables|/Game/VigilanteContent/Projectiles/East_Bomb_KAB500/BPA_East_Bomb_KAB500.BPA_East_Bomb_KAB500_C|SetFin1Angle (Variables|Default|GetAnimInstance) (Math|Float|MapRangeClamped Fin1Angle -1.0 1.0 -45.0 45.0)))

(event Custom|SetFin2Angle
  (params (Fin2Angle :type Float%20%28single-precision%29))
  (Variables|/Game/VigilanteContent/Projectiles/East_Bomb_KAB500/BPA_East_Bomb_KAB500.BPA_East_Bomb_KAB500_C|SetFin2Angle (Variables|Default|GetAnimInstance) (Math|Float|MapRangeClamped Fin2Angle -1.0 1.0 -45.0 45.0)))

(event Custom|SetFin3Angle
  (params (SetFin3Angle :type Float%20%28single-precision%29))
  (Variables|/Game/VigilanteContent/Projectiles/East_Bomb_KAB500/BPA_East_Bomb_KAB500.BPA_East_Bomb_KAB500_C|SetFin3Angle (Variables|Default|GetAnimInstance) (Math|Float|MapRangeClamped SetFin3Angle -1.0 1.0 -45.0 45.0)))

(event Custom|SetFin4Angle
  (params (SetFin4Angle :type Float%20%28single-precision%29))
  (Variables|/Game/VigilanteContent/Projectiles/East_Bomb_KAB500/BPA_East_Bomb_KAB500.BPA_East_Bomb_KAB500_C|SetFin4Angle (Variables|Default|GetAnimInstance) (Math|Float|MapRangeClamped SetFin4Angle -1.0 1.0 -45.0 45.0)))

(event EventBeginPlay
  (bind _asbpa_east_bomb_kab500 (Utilities|Casting|CastToBPA_East_Bomb_KAB500 (Components|SkeletalMesh|GetAnimInstance (Variables|Default|GetSkeletalMesh))))
  (Variables|Default|SetAnimInstance _asbpa_east_bomb_kab500))

(fn ConstructionScript)