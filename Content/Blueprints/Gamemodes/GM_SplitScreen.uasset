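; Split-screen game mode that spawns a Ford car for each local player at level start.
; BeginPlay reads every PlayerStart tag as a number: positive values create a local player with that ID, others use player 0, and each possesses a car spawned there.
; Events for adding and removing players as input devices connect or disconnect exist, but their binding and startup call are disconnected, so that path is inactive.
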(event Custom|OnInputDeviceConnectionChange_Event
  (params (NewConnectionState :type EInputDeviceConnectionState%20Enum :default "Invalid") (PlatformUserId :type Platform%20User%20Id%20Structure) (InputDeviceId :type Input%20Device%20Id%20Structure))
  (if (!= (Math|Conversions|ToInteger(Byte) (Utilities|String|ToString(Integer) InputDeviceId)) 0)
    (switch Utilities|FlowControl|Switch|SwitchonEInputDeviceConnectionState NewConnectionState
      (:Disconnected
        (bind _returnvalue (Class|InputDeviceLibrary|GetPlayerControllerfromInputDevice InputDeviceId))
        (Class|GameplayStatics|RemovePlayer _returnvalue true))
      (:Connected
        (Class|GameplayStatics|CreatePlayer -1)))))

(event Custom|ConnectExistingDevices
  (bind _outinputdevices (Class|InputDeviceLibrary|GetAllInputDevices))
  (for (_ _array_index) _outinputdevices
    (if (!= _array_index 0)
      (Class|GameplayStatics|CreatePlayer -1))))

(event EventBeginPlay
  (bind _returnvalue (Game|GetPlayerController 0))
  (bind _outactors (Actor|GetAllActorsOfClass "/Script/Engine.PlayerStart"))
  (for _array_element _outactors
    (if (> (Math|Conversions|ToInteger(Byte) (Utilities|String|ToString(Name) (Variables|/Script/Engine.PlayerStart|GetPlayerStartTag _array_element))) 0)
      (bind _returnvalue_2 (Class|GameplayStatics|CreatePlayer (Math|Conversions|ToInteger(Byte) (Utilities|String|ToString(Name) (Variables|/Script/Engine.PlayerStart|GetPlayerStartTag _array_element)))))
      (bind _returnvalue_3 (Game|SpawnActorfromClass "/Game/Blueprints/Car/BP_FordCar.BP_FordCar_C" (Transformation|GetActorTransform _array_element) "Undefined" "MultiplyWithRoot" 0 0))
      (Pawn|Possess _returnvalue_2 _returnvalue_3)
      (else
        (bind _returnvalue_4 (Game|SpawnActorfromClass "/Game/Blueprints/Car/BP_FordCar.BP_FordCar_C" (Transformation|GetActorTransform _array_element) "Undefined" "MultiplyWithRoot" _returnvalue 0))
        (Pawn|Possess _returnvalue _returnvalue_4)))))

(fn ConstructionScript)