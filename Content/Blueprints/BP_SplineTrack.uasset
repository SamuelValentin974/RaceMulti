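; BP_SplineTrack is an actor that moves a list of actors continuously along its spline, evenly spaced by an offset.
; The construction script places the actors at their spaced starting points along the spline.
; At BeginPlay a timeline, with its play rate set from TimeLength, drives distance along the spline, setting each actor's location and rotation.
; Distances past the spline end wrap to the start, and the timeline restarts on finish to loop.
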(event Custom|PlayTime
  (bind _spline (Variables|Default|GetSpline))
  (bind _spline_2 (Variables|Default|GetSpline))
  (bind _returnvalue (Spline|GetSplineLength _spline))
  (bind _newtrack_0 (Timeline|Timeline PlayFromStart)
    (:Update
      (for (_array_element _array_index) (Variables|Default|GetActors)
        (bind _output_get (Variables|Default|SetDistanceAlongSpline (+ (Math|Float|Lerp 0.0 (Spline|GetSplineLength (Variables|Default|GetSpline)) _newtrack_0) (* _array_index (Variables|Default|GetOffsetBtwActor)))))
        (if (> _output_get _returnvalue)
          (Variables|Default|SetDistanceAlongSpline (- (Variables|Default|GetDistanceAlongSpline) _returnvalue)))
        (Transformation|SetActorLocationAndRotation _array_element (Spline|GetLocationatDistanceAlongSpline _spline_2 (Variables|Default|GetDistanceAlongSpline) "World") (Spline|GetRotationatDistanceAlongSpline _spline_2 (Variables|Default|GetDistanceAlongSpline) "World"))))
    (:Finished
      (CallFunction|PlayTime))))

(event EventBeginPlay
  (Components|Timeline|SetPlayRate (Variables|Default|GetTimeline) (/ 1.0 (Variables|Default|GetTimeLength)))
  (CallFunction|PlayTime))

(event Collision|EventActorBeginOverlap
  (params (OtherActor :type Actor%20Object%20Reference)))

(event EventTick
  (params (DeltaSeconds :type Float%20%28single-precision%29)))

(fn ConstructionScript
  (bind _spline (Variables|Default|GetSpline))
  (for (_array_element _array_index) (Variables|Default|GetActors)
    (Transformation|SetActorLocationAndRotation _array_element (Spline|GetLocationatDistanceAlongSpline _spline (* (Variables|Default|GetOffsetBtwActor) _array_index) "World") (Spline|GetRotationatDistanceAlongSpline _spline (* (Variables|Default|GetOffsetBtwActor) _array_index) "World"))))