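; BP_CheckPoint is a one-shot checkpoint that records respawn data on the BP_FordCar that drives through it.
; When the car overlaps its Box, the checkpoint disables collision, hides itself and calls the HitCheckPoints dispatcher.
; If its CheckPointsIndex exceeds the car's last index, it stores its own world transform, the car's rotation and the new index on the car.
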(event OnComponentBeginOverlap(Box)
  (params (OverlappedComponent :type Primitive%20Component%20Object%20Reference) (OtherActor :type Actor%20Object%20Reference) (OtherComp :type Primitive%20Component%20Object%20Reference) (OtherBodyIndex :type Integer) (bFromSweep :type Boolean) (SweepResult :type Hit%20Result%20Structure%20%28by%20ref%29))
  (bind _asbp_ford_car (Utilities|Casting|CastToBP_FordCar OtherActor))
  (Variables|Default|SetAs%20BP%20Ford%20Car _asbp_ford_car)
  (Collision|SetCollisionEnabled (Variables|Default|GetCube) "NoCollision")
  (Collision|SetCollisionEnabled (Variables|Default|GetBox) "NoCollision")
  (Rendering|SetActorHiddenInGame true)
  (Default|CallHitCheckPoints)
  (if (> (Variables|Default|GetCheckPointsIndex) (Variables|/Game/Blueprints/Car/BP_FordCar.BP_FordCar_C|GetLastCheckPointIndex (Variables|Default|GetAs%20BP%20Ford%20Car)))
    (Variables|/Game/Blueprints/Car/BP_FordCar.BP_FordCar_C|SetLastCheckPointTransform (Variables|Default|GetAs%20BP%20Ford%20Car) (Transformation|GetWorldTransform (Variables|Default|GetDefaultSceneRoot)))
    (Variables|/Game/Blueprints/Car/BP_FordCar.BP_FordCar_C|SetLastRotation (Variables|Default|GetAs%20BP%20Ford%20Car) (Transformation|GetActorRotation (Variables|Default|GetAs%20BP%20Ford%20Car)))
    (Variables|/Game/Blueprints/Car/BP_FordCar.BP_FordCar_C|SetLastCheckPointIndex (Variables|Default|GetAs%20BP%20Ford%20Car) (Variables|Default|GetCheckPointsIndex))))

(event EventBeginPlay
  (Collision|SetCollisionEnabled (Variables|Default|GetCube) "QueryOnly")
  (Collision|SetCollisionEnabled (Variables|Default|GetBox) "QueryOnly"))

(fn ConstructionScript)