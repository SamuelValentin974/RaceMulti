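; Spline-driven barrier actor that lines a path with Chaos Geometry Collection pieces, apparently for destructible barriers.
; The construction script measures the Mesh bounding box along X and uses that length as the spacing along the spline.
; At each step it adds a collision-enabled Geometry Collection component, rotated to the spline tangent rather than deformed along the curve.
; The event graph has no active logic, including an empty spline hit event.
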(event OnComponentHit(Spline)
  (params (HitComponent :type Primitive%20Component%20Object%20Reference) (OtherActor :type Actor%20Object%20Reference) (OtherComp :type Primitive%20Component%20Object%20Reference) (NormalImpulse :type Vector :default "0, 0, 0") (Hit :type Hit%20Result%20Structure%20%28by%20ref%29)))

(event EventBeginPlay)

(event Collision|EventActorBeginOverlap
  (params (OtherActor :type Actor%20Object%20Reference)))

(event EventTick
  (params (DeltaSeconds :type Float%20%28single-precision%29)))

(fn ConstructionScript
  (bind _mesh (Variables|Default|GetMesh))
  (bind _spline (Variables|Default|GetSpline))
  (bind _returnvalue (StaticMesh|GetBoundingBox _mesh))
  (bind _output_get (Variables|Default|SetXlength (.x (+ (Math|Vector|VectorGetAbs (.min _returnvalue)) (Math|Vector|VectorGetAbs (.max _returnvalue))))))
  (for _index (range 0 (Math|Float|Truncate (/ (Spline|GetSplineLength (Variables|Default|GetSpline)) _output_get)))
    (bind _returnvalue_2 (AddComponent|AddGeometryCollectionComponent false))
    (Collision|SetCollisionEnabled _returnvalue_2 "QueryAndPhysics")
    (Transformation|SetRelativeLocationAndRotation _returnvalue_2 (Spline|GetLocationatDistanceAlongSpline _spline (* _index (Variables|Default|GetXlength)) "Local") (Math|Rotator|MakeRotfromX (Math|Vector|ClampVectorSize (Spline|GetTangentatDistanceAlongSpline _spline (* _index (Variables|Default|GetXlength)) "Local") 0.0 (Variables|Default|GetXlength))) false false)))