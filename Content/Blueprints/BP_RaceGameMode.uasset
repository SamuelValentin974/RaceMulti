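; Racing game mode that runs the start countdown, race and lap timing, lap progress and the finish sequence.
; BeginPlay starts a timer-driven countdown that locks cars until GO, then timelines drive the race and lap clocks.
; Checkpoint hits are counted and re-armed after a completed lap; UpdateLaps records split times or ends the race.
; The finish hides the HUD, blends to a cine camera, speeds up time and shows the results widget.
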(event Custom|StartRaceTimer
  (bind _time (Timeline|RaceTimeline PlayFromStart)
    (:Update
      (Variables|Lap/RaceText|SetRaceTime (Utilities|TimeConverter _time)))))

(event Custom|FinishRaceTimer
  (bind _time (Timeline|RaceTimeline Stop)
    (:Update
      (Variables|Lap/RaceText|SetRaceTime (Utilities|TimeConverter _time)))))

(event Custom|StartLapTimer
  (bind _time (Timeline|LapTimeLine PlayFromStart)
    (:Update
      (Variables|Lap/RaceText|SetLapTime (Utilities|TimeConverter _time)))))

(event Custom|EndLapTimer
  (bind _time (Timeline|LapTimeLine Stop)
    (:Update
      (Variables|Lap/RaceText|SetLapTime (Utilities|TimeConverter _time)))))

(event Custom|StartRaceCountDown
  (Variables|Default|SetCarLock? true)
  (Variables|Default|SetCountDown 4.0)
  (Utilities|Time|SetTimerbyFunctionName 0 "CountDownTick" 1.0 true))

(event Custom|CountDownTick
  (bind _countdown (Variables|Default|GetCountDown))
  (bind _result (Math|Float|DecrementFloat (Variables|Default|GetCountDown))
    (:%20%20
      (Variables|Lap/RaceText|SetCountDownText (Utilities|Text|ToText(Float) _result "HalfToEven"))
      (if (>= _countdown 1.0)
        (Audio|PlaySound2D "/Game/UI/SFX/Effects/short-beep-tone-47916.short-beep-tone-47916" 1.0 1.0 0.0 0 0)
        (elif (== _countdown 0.0)
          (Variables|Lap/RaceText|SetCountDownText "GO !")
          (Audio|PlaySound2D "/Game/UI/SFX/Effects/short-beep-tone-47916.short-beep-tone-47916" 1.0 1.2 0.0 0 0)
          (Utilities|Time|ClearTimerbyFunctionName 0 "CountDownTick")
          (Variables|Default|SetCarLock? false)
          (CallFunction|StartLapTimer)
          (Utilities|FlowControl|DoOnce false
            (:Completed
              (CallFunction|StartRaceTimer)
              (Variables|Default|SetRaceStart? true)
              (Utilities|FlowControl|Delay 2.0)
              (Variables|Lap/RaceText|SetCountDownText ""))))))))

(event Custom|UpdateLaps
  (bind _lapscompleted (Variables|Default|GetLapsCompleted))
  (bind _lapsrequired (Variables|Default|GetLapsRequired))
  (bind _laptime (Variables|Lap/RaceText|GetLapTime))
  (Variables|Lap/RaceText|SetLap%20Text (Utilities|LapsText _lapscompleted _lapsrequired))
  (if (> _lapscompleted _lapsrequired)
    (Variables|Default|SetRaceEnd? true)
    (CallFunction|RaceFinished)
    (else
      (Variables|Default|SetLapCompleted? true)
      (switch int (- (Variables|Default|GetLapsCompleted) 1)
        (:1
          (Variables|Lap/RaceText|SetLap1 _laptime))
        (:2
          (Variables|Lap/RaceText|SetLap2 _laptime))
        (:3
          (Variables|Lap/RaceText|SetLap3 _laptime))))))

(event Custom|Hit
  (bind _checkpointcount (Variables|Default|GetCheckPointCount))
  (Development|PrintString "Hit checkpoints")
  (Math|Integer|IncrementInt _checkpointcount
    (:%20%20
      (if (>= _checkpointcount (Variables|Default|GetNbCheckPoints))
        (Utilities|Time|SetTimerbyEvent (delegate Custom|ResetCheckPoints) 1.0 true)))))

(event Custom|ResetCheckPoints
  (if (Variables|Default|GetLapCompleted?)
    (Variables|Default|SetLapCompleted? false)
    (for _array_element (Variables|Default|GetCheckPoints)
      (Collision|SetCollisionEnabled (Variables|/Game/Blueprints/BP_CheckPoint.BP_CheckPoint_C|GetCube _array_element) "QueryOnly")
      (Collision|SetCollisionEnabled (Variables|/Game/Blueprints/BP_CheckPoint.BP_CheckPoint_C|GetBox _array_element) "QueryOnly")
      (Rendering|SetActorHiddenInGame _array_element false)
      (Variables|Default|SetCheckPointCount 0))))

(event Custom|RaceFinished
  (bind _returnvalue (Game|GetPlayerController 0))
  (CallFunction|FinishRaceTimer)
  (bind _foundwidgets (Widget|GetAllWidgetsOfClass "/Game/UI/Widget/WP_PlayerHud.WP_PlayerHud_C" true))
  (Utilities|IsValid (Utilities|Array|Get(acopy) _foundwidgets)
    (:Is%20Valid
      (Widget|SetVisibility (Utilities|Array|Get(acopy) _foundwidgets) "Hidden")
      (Input|SetInputModeUIOnly _returnvalue 0 "DoNotLock" false)
      (Variables|/Script/Engine.PlayerController|SetbShowMouseCursor _returnvalue true)
      (bind _returnvalue_2 (Actor|GetActorOfClass "/Script/CinematicCamera.CineCameraActor"))
      (Game|Player|SetViewTargetwithBlend _returnvalue _returnvalue_2 0.0 "VTBlend_Linear" 0.0 false)
      (Utilities|Time|SetGlobalTimeDilation 5.0)
      (Utilities|FlowControl|Delay 3.0)
      (bind _returnvalue_3 (UserInterface|CreateWidget "/Game/UI/Widget/WBP_FinishRace.WBP_FinishRace_C"))
      (UserInterface|Viewport|AddtoViewport _returnvalue_3 0)
      (Widget|SetVisibility _returnvalue_3 "Visible"))))

(event EventBeginPlay
  (bind _output_get (Variables|Default|SetLapsRequired (Variables|Default|GetLapsRequired)))
  (bind _output_get_2 (Variables|Default|SetLapsCompleted 3))
  (Variables|Lap/RaceText|SetLap%20Text (Utilities|LapsText _output_get_2 _output_get))
  (Variables|Lap/RaceText|SetCountDownText "Ready ?")
  (Utilities|FlowControl|Delay 4.0)
  (CallFunction|StartRaceCountDown)
  (bind _outactors (Actor|GetAllActorsOfClass "/Game/Blueprints/BP_CheckPoint.BP_CheckPoint_C"))
  (bind _output_get_3 (Variables|Default|SetCheckPoints _outactors))
  (bind _output_get_4 (Variables|Default|SetNbCheckPoints (Utilities|Array|Length _output_get_3)))
  (for _array_element (Variables|Default|GetCheckPoints)
    (EventDispatchers|BindEventtoHitCheckPoints _array_element (delegate Custom|Hit))))

(fn ConstructionScript)