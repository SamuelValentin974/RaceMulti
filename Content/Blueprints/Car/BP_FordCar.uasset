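; Player-drivable Chaos wheeled car mapping Enhanced Input to throttle, brake, steering, handbrake, upright reset and camera controls.
; Tick adjusts airborne angular damping, recenters the spring arm, feeds RPM to engine audio, triggers off-throttle backfires and holds neutral when stopped on handbrake.
; Handbrake cuts rear wheel friction, restored by a timeline on release.
; Skid-based counter-steer and friction logic exists but is never called; BrakeLights is an empty stub.
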(event Custom|InterpsToOriginalRotation
  (Transformation|SetRelativeRotation (Variables|Default|GetSpringArm) (Math|Rotator|MakeRotator 0.0 0.0 (Math|Interpolation|FInterpTo (.yaw (Variables|/Script/Engine.SceneComponent|GetRelativeRotation (Variables|Default|GetSpringArm))) 0.0 (Utilities|Time|GetWorldDeltaSeconds) 1.0)) false false))

(event Custom|CounterSteer
  ;[1 1 1] Comment
  (CallFunction|DetectLeftSkid)
  (CallFunction|DetectRightSkid)
  (if (Variables|Default|GetLeftSkidding)
    (Variables|Default|SetSteeringModif (Math|Float|Lerp (stale Input|EnhancedActionEvents|EnhancedInputActionIA_Steering ActionValue) (* (stale Input|EnhancedActionEvents|EnhancedInputActionIA_Steering ActionValue) (Variables|Default|GetSteeringMult)) 0.25))
    (Class|ChaosWheeledVehicleMovementComponent|SetMaxEngineTorque (Variables|Default|GetCWVM_Ref) 2e+03)
    (elif (Variables|Default|GetRigthSkidding)
      (Variables|Default|SetSteeringModif (Math|Float|Lerp (stale Input|EnhancedActionEvents|EnhancedInputActionIA_Steering ActionValue) (* (stale Input|EnhancedActionEvents|EnhancedInputActionIA_Steering ActionValue) (Variables|Default|GetSteeringMult)) 0.25))
      (Class|ChaosWheeledVehicleMovementComponent|SetMaxEngineTorque (Variables|Default|GetCWVM_Ref) 2e+03))))

(event Custom|DetectRightSkid
  (bind _cwvm_ref (Variables|Default|GetCWVM_Ref))
  (bind _returnvalue (Class|ChaosWheeledVehicleMovementComponent|GetWheelState _cwvm_ref 1))
  (bind _skidmagnitude (Class|ChaosWheeledVehicleMovementComponent|BreakWheelStatus _returnvalue))
  ;[1 1 1] Comment
  (Development|PrintString (Utilities|String|ToString(Float) _skidmagnitude))
  (if (< _skidmagnitude -4e+02)
    (Variables|Default|SetRigthSkidding true)
    (Variables|Default|SetFrictionFrontCurrent (Math|Float|Clamp(Float) _skidmagnitude 0.0 4.5))
    (else
      (Variables|Default|SetRigthSkidding false)
      ;;[1 1 1] Comment
      (Variables|Default|SetfrictionRearCurent (Math|Float|Lerp (Variables|Default|GetfrictionRearCurent) (Variables|Default|GetFRearBase) 0.01))
      (Variables|Default|SetFrictionFrontCurrent (Math|Float|Lerp (Variables|Default|GetFrictionFrontCurrent) (Variables|Default|GetFFrontBase) 0.01))))
  (Class|ChaosWheeledVehicleMovementComponent|SetWheelFrictionMultiplier (Variables|Default|GetCWVM_Ref) 0 (Variables|Default|GetFrictionFrontCurrent))
  (Class|ChaosWheeledVehicleMovementComponent|SetWheelFrictionMultiplier (Variables|Default|GetCWVM_Ref) 1 (Variables|Default|GetFrictionFrontCurrent))
  (Class|ChaosWheeledVehicleMovementComponent|SetWheelFrictionMultiplier (Variables|Default|GetCWVM_Ref) 2 (Variables|Default|GetfrictionRearCurent))
  (Class|ChaosWheeledVehicleMovementComponent|SetWheelFrictionMultiplier (Variables|Default|GetCWVM_Ref) 3 (Variables|Default|GetfrictionRearCurent))
  (Utilities|FlowControl|Delay 1.0)
  (Variables|Default|SetfrictionRearCurent (Math|Float|Lerp (Variables|Default|GetfrictionRearCurent) (Variables|Default|GetFRearBase) 0.01))
  (Variables|Default|SetFrictionFrontCurrent (Math|Float|Lerp (Variables|Default|GetFrictionFrontCurrent) (Variables|Default|GetFFrontBase) 0.01)))

(event Custom|DetectLeftSkid
  (bind _cwvm_ref (Variables|Default|GetCWVM_Ref))
  (bind _returnvalue (Class|ChaosWheeledVehicleMovementComponent|GetWheelState _cwvm_ref))
  (bind _skidmagnitude (Class|ChaosWheeledVehicleMovementComponent|BreakWheelStatus _returnvalue))
  ;[1 1 1] Comment
  (Development|PrintString (Utilities|String|ToString(Float) _skidmagnitude))
  (if (> _skidmagnitude 4e+02)
    (Variables|Default|SetLeftSkidding true)
    (Variables|Default|SetfrictionRearCurent (Math|Float|Clamp(Float) _skidmagnitude 2.0 4.0))
    (else
      (Variables|Default|SetLeftSkidding false)
      ;;[1 1 1] Comment
      (Variables|Default|SetfrictionRearCurent (Math|Float|Lerp (Variables|Default|GetfrictionRearCurent) (Variables|Default|GetFRearBase) 0.01))
      (Variables|Default|SetFrictionFrontCurrent (Math|Float|Lerp (Variables|Default|GetFrictionFrontCurrent) (Variables|Default|GetFFrontBase) 0.01))))
  (Class|ChaosWheeledVehicleMovementComponent|SetWheelFrictionMultiplier (Variables|Default|GetCWVM_Ref) 0 (Variables|Default|GetFrictionFrontCurrent))
  (Class|ChaosWheeledVehicleMovementComponent|SetWheelFrictionMultiplier (Variables|Default|GetCWVM_Ref) 1 (Variables|Default|GetFrictionFrontCurrent))
  (Class|ChaosWheeledVehicleMovementComponent|SetWheelFrictionMultiplier (Variables|Default|GetCWVM_Ref) 2 (Variables|Default|GetfrictionRearCurent))
  (Class|ChaosWheeledVehicleMovementComponent|SetWheelFrictionMultiplier (Variables|Default|GetCWVM_Ref) 3 (Variables|Default|GetfrictionRearCurent))
  (Utilities|FlowControl|Delay 1.0)
  (Variables|Default|SetfrictionRearCurent (Math|Float|Lerp (Variables|Default|GetfrictionRearCurent) (Variables|Default|GetFRearBase) 0.01))
  (Variables|Default|SetFrictionFrontCurrent (Math|Float|Lerp (Variables|Default|GetFrictionFrontCurrent) (Variables|Default|GetFFrontBase) 0.01)))

(event Input|EnhancedActionEvents|EnhancedInputActionIA_Throttle
  (params (ActionValue :type Float%20%28double-precision%29) (ElapsedSeconds :type Float%20%28double-precision%29) (TriggeredSeconds :type Float%20%28double-precision%29) (InputAction :type Input%20Action%20Object%20Reference :default "/Game/Input/Actions/IA_Throttle.IA_Throttle"))
  (:Triggered
    (Class|ChaosVehicleMovementComponent|SetThrottleInput (Variables|Default|GetVehicleMovementComponent) ActionValue :!label _label)
    (if (or (Variables|Default|GetLeftSkidding) (Variables|Default|GetRigthSkidding))
      (Variables|Default|SetfrictionRearCurent (- (Variables|Default|GetfrictionRearCurent) 2.0))
      (Variables|Default|SetFrictionFrontCurrent (- (Variables|Default|GetFrictionFrontCurrent) 2.0))))
  (:Completed
    (goto _label)))

(event Input|EnhancedActionEvents|EnhancedInputActionIA_Brake
  (params (ActionValue :type Float%20%28double-precision%29) (ElapsedSeconds :type Float%20%28double-precision%29) (TriggeredSeconds :type Float%20%28double-precision%29) (InputAction :type Input%20Action%20Object%20Reference :default "/Game/Input/Actions/IA_Brake.IA_Brake"))
  (:Triggered
    (Class|ChaosVehicleMovementComponent|SetBrakeInput (Variables|Default|GetVehicleMovementComponent) ActionValue :!label _label)
    (CallFunction|BrakeLights false))
  (:Started
    (CallFunction|BrakeLights true))
  (:Completed
    (goto _label)))

(event Input|EnhancedActionEvents|EnhancedInputActionIA_Steering
  (params (ActionValue :type Float%20%28double-precision%29) (ElapsedSeconds :type Float%20%28double-precision%29) (TriggeredSeconds :type Float%20%28double-precision%29) (InputAction :type Input%20Action%20Object%20Reference :default "/Game/Input/Actions/IA_Steering.IA_Steering"))
  ;[1 1 1] Comment
  (:Triggered
    (Variables|Default|SetSteeringModif ActionValue :!label _label)
    (Class|ChaosVehicleMovementComponent|SetSteeringInput (Variables|Default|GetCWVM_Ref) (Variables|Default|GetSteeringModif)))
  (:Started
    (goto _label))
  (:Ongoing
    (goto _label))
  (:Completed
    (goto _label)))

(event Input|EnhancedActionEvents|EnhancedInputActionIA_HandBrake
  (params (ActionValue :type Boolean) (ElapsedSeconds :type Float%20%28double-precision%29) (TriggeredSeconds :type Float%20%28double-precision%29) (InputAction :type Input%20Action%20Object%20Reference :default "/Game/Input/Actions/IA_HandBrake.IA_HandBrake"))
  (bind _cwvm_ref (Variables|Default|GetCWVM_Ref))
  (:Triggered
    (Class|ChaosWheeledVehicleMovementComponent|SetWheelFrictionMultiplier _cwvm_ref 2 0.5)
    (Class|ChaosWheeledVehicleMovementComponent|SetWheelFrictionMultiplier _cwvm_ref 3 0.5)
    (Class|ChaosVehicleMovementComponent|SetHandbrakeInput _cwvm_ref ActionValue :!label _label))
  (:Completed
    (bind _newtrack_0 (Timeline|Timeline PlayFromStart)
      (:Update
        (Class|ChaosWheeledVehicleMovementComponent|SetWheelFrictionMultiplier _cwvm_ref 2 _newtrack_0)
        (Class|ChaosWheeledVehicleMovementComponent|SetWheelFrictionMultiplier _cwvm_ref 3 _newtrack_0)
        (goto _label)))))

(event Input|EnhancedActionEvents|EnhancedInputActionIA_Camera
  (params (ActionValue :type Float%20%28double-precision%29) (ElapsedSeconds :type Float%20%28double-precision%29) (TriggeredSeconds :type Float%20%28double-precision%29) (InputAction :type Input%20Action%20Object%20Reference :default "/Game/Input/Actions/IA_Camera.IA_Camera"))
  (Transformation|AddLocalRotation (Variables|Default|GetSpringArm) (Math|Rotator|MakeRotator 0.0 0.0 ActionValue) false false))

(event Input|EnhancedActionEvents|EnhancedInputActionIA_Reset
  (params (ActionValue :type Boolean) (ElapsedSeconds :type Float%20%28double-precision%29) (TriggeredSeconds :type Float%20%28double-precision%29) (InputAction :type Input%20Action%20Object%20Reference :default "/Game/VehicleTemplate/Input/Actions/IA_Reset.IA_Reset"))
  (Transformation|SetActorTransform (Math|Transform|MakeTransform (+ (Transformation|GetActorLocation) "0,0,50.000000") (Math|Rotator|MakeRotator 0.0 0.0 (.yaw (Transformation|GetActorRotation)))) false true)
  (Class|PrimitiveComponent|SetPhysicsAngularVelocityinDegrees (Variables|Character|GetMesh) "0, 0, 0" false "None")
  (Physics|SetPhysicsLinearVelocity (Variables|Character|GetMesh) "0, 0, 0" false "None"))

(event Input|EnhancedActionEvents|EnhancedInputActionIA_ToggleCamera
  (params (ActionValue :type Boolean) (ElapsedSeconds :type Float%20%28double-precision%29) (TriggeredSeconds :type Float%20%28double-precision%29) (InputAction :type Input%20Action%20Object%20Reference :default "/Game/VehicleTemplate/Input/Actions/IA_ToggleCamera.IA_ToggleCamera"))
  (Components|Activation|Deactivate (Variables|Default|GetBackCamera))
  (Utilities|FlowControl|FlipFlop
    (:A
      (Components|Activation|Activate (Variables|Default|GetFrontCamera) false))
    (:B
      (Components|Activation|Activate (Variables|Default|GetBackCamera) false))))

(event EventTick
  (params (DeltaSeconds :type Float%20%28single-precision%29))
  (Class|PrimitiveComponent|SetAngularDamping (Variables|Character|GetMesh) (Math|Float|SelectFloat 0.0 3.0 (AI|Components|NavMovement|IsMovingonGround (Variables|Default|GetCWVM_Ref))))
  (CallFunction|InterpstoOriginalRotation)
  (Audio|Parameter|SetFloatParameter (Variables|Default|GetEngine) "RPM" (Math|Float|MapRangeClamped (Class|ChaosWheeledVehicleMovementComponent|GetEngineRotationSpeed (Variables|Default|GetCWVM_Ref)) 1e+03 7.9e+03 0.0 1.0) :!class /Script/AudioExtensions.AudioParameterControllerInterface)
  (Utilities|FlowControl|Sequence
    (:then_0
      (CallFunction|NeutralAcc))
    (:then_1
      (CallFunction|EngineSound))))

(event EventBeginPlay
  (bind _aschaos_wheeled_vehicle_movement_component (Utilities|Casting|CastToChaosWheeledVehicleMovementComponent (Variables|Default|GetVehicleMovementComponent)))
  (Variables|Default|SetCWVM_Ref _aschaos_wheeled_vehicle_movement_component))

(fn ConstructionScript)

(fn BrakeLights
  (params (Is%20Braking :type Boolean)))

(fn NeutralAcc
  (bind _cwvm_ref (Variables|Default|GetCWVM_Ref))
  (bind _cwvm_ref_2 (Variables|Default|GetCWVM_Ref))
  (bind _returnvalue (Class|ChaosVehicleMovementComponent|GetThrottleInput _cwvm_ref))
  (if (and (Class|ChaosVehicleMovementComponent|GetHandbrakeInput _cwvm_ref) (< (Class|ChaosVehicleMovementComponent|GetForwardSpeedMPH _cwvm_ref) 2.0))
    (Class|ChaosVehicleMovementComponent|SetTargetGear _cwvm_ref_2 0 false)
    (Class|ChaosVehicleMovementComponent|SetUseAutomaticGears _cwvm_ref_2 false)
    (else
      (Class|ChaosVehicleMovementComponent|SetUseAutomaticGears _cwvm_ref_2 true))))

(fn EngineSound
  (bind _cwvm_ref (Variables|Default|GetCWVM_Ref))
  (bind _ns_backfire (Variables|Default|GetNS_Backfire))
  (bind _returnvalue (Class|ChaosVehicleMovementComponent|GetThrottleInput _cwvm_ref))
  (if (and (< _returnvalue 0.2) (> (Class|ChaosWheeledVehicleMovementComponent|GetEngineRotationSpeed _cwvm_ref) 5e+03))
    (Components|Activation|Activate _ns_backfire false)
    (Audio|SpawnSoundatLocation 0 (Transformation|GetSocketLocation _ns_backfire "Echap1") "0, 0, 0" 1.0 1.0 0.0 0 0)
    (else
      (Components|Activation|Deactivate (Variables|Default|GetNS_Backfire1)))))

(fn Steering
  (params (Value :type Float%20%28double-precision%29)))