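; BP_StartLine is the start line trigger that counts completed laps in the race.
; It caches the player controller and race game mode at BeginPlay, then reacts to overlaps on its Box.
; A Skip flag, when set, swallows one crossing.
; Otherwise, if the race has started and the checkpoint count equals the required number, it increments the game mode's completed laps, updates them and starts a lap.
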(event OnComponentBeginOverlap(Box)
  (params (OverlappedComponent :type Primitive%20Component%20Object%20Reference) (OtherActor :type Actor%20Object%20Reference) (OtherComp :type Primitive%20Component%20Object%20Reference) (OtherBodyIndex :type Integer) (bFromSweep :type Boolean) (SweepResult :type Hit%20Result%20Structure%20%28by%20ref%29))
  (bind _as_bp_race_game_mode (Variables|Default|GetAs%20BP%20Race%20Game%20Mode))
  (bind _as_bp_race_game_mode_2 (Variables|Default|GetAs%20BP%20Race%20Game%20Mode))
  (bind _as_bp_race_game_mode_3 (Variables|Default|GetAs%20BP%20Race%20Game%20Mode))
  (if (Variables|Default|Getskip?)
    (Variables|Default|Setskip? false)
    (elif (Variables|/Game/Blueprints/BP_RaceGameMode.BP_RaceGameMode_C|GetRaceStart? _as_bp_race_game_mode_2)
      (if (== (Variables|/Game/Blueprints/BP_RaceGameMode.BP_RaceGameMode_C|GetCheckPointCount _as_bp_race_game_mode) (Variables|/Game/Blueprints/BP_RaceGameMode.BP_RaceGameMode_C|GetNbCheckPoints _as_bp_race_game_mode))
        (Math|Integer|IncrementInt (Variables|/Game/Blueprints/BP_RaceGameMode.BP_RaceGameMode_C|GetLapsCompleted _as_bp_race_game_mode_2)
          (:%20%20
            (Default|UpdateLaps _as_bp_race_game_mode_3)
            (Default|StartLap _as_bp_race_game_mode_3)))))))

(event EventBeginPlay
  (bind _asbp_player_controller (Utilities|Casting|CastToBP_PlayerController (Game|GetPlayerController 0)))
  (Variables|Default|SetAs%20BP%20Player%20Controller _asbp_player_controller)
  (bind _asbp_race_game_mode (Utilities|Casting|CastToBP_RaceGameMode (Game|GetGameMode)))
  (Variables|Default|SetAs%20BP%20Race%20Game%20Mode _asbp_race_game_mode))

(fn ConstructionScript)